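; BP_MainRunner is the runner player character, handling lane changes, sliding, power-ups and the selected character's mesh.
; Timelines drive lane-change updates and lerp capsule half-height and mesh offset for slides.
; Magnet, shield and high-jump events toggle their effects and report to the GameMode's HUD, with magnet and shield using lazily cached child actors.
; The mesh comes from the character index saved in the "Menu" slot, defaulting to the first.
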(event `self.ChangeLane`
  (bind (_direction _newtrack_0) (`Timeline|LaneChangeSmooth` :!via `PlayFromStart`)
    (:`Update`
      (`self.ChangeLaneUpdate` _newtrack_0))
    (:`Finished`
      (`self.ChangeLaneFinished`))))

(event `self.TimeSlide`
  (params (value :type Boolean))
  (if value
    (bind (_direction _capusle) (`Timeline|Slide` :!via `PlayFromStart` :!label _label)
      (:`Update`
        (`self.mesh&CapulseHeight` _capusle _capusle)))))

(event `SlideEndD`
  (goto _label :!via `ReverseFromEnd`))

(event `self.CharacterSelected`
  (`self.Character`))

(event `/Game/Main/BP/interface/BPI_Player.Magnet`
  (`self.As BP Magnet Powerup`
    (:`then`
      _)
    (:`else`
      (bind _asbp_magnet_powerup (cast `/Game/Main/BP/Powerup/BP_MagnetPowerup` (`ChildActorComponent.ChildActor` (`self.BP_MagnetPowerup`))))
      (set `self.As BP Magnet Powerup` _asbp_magnet_powerup)))
  (`/Game/Main/BP/Powerup/BP_MagnetPowerup.MagnetPowerup` (`self.As BP Magnet Powerup`) true)
  (`SceneComponent.SetVisibility` (`self.Magnet_metal`) true false)
  (`SceneComponent.SetVisibility` (`self.Magnet_magnet1`) true false)
  ;[1 1 1] End to zero for progress
  (`GameHud.MagnetPowerupupdates` (`GMRunner.GameHud` (`self.MainGameMode`)) 0.0 (`self.MagnetDuration`)))

(event `/Game/Main/BP/interface/BPI_Player.DeactiveMagnet`
  (`/Game/Main/BP/Powerup/BP_MagnetPowerup.MagnetPowerup` (`self.As BP Magnet Powerup`) false)
  (`SceneComponent.SetVisibility` (`self.Magnet_magnet1`) false false)
  (`SceneComponent.SetVisibility` (`self.Magnet_metal`) false false))

(event `/Game/Main/BP/interface/BPI_Player.HighJumpPowerUpI`
  (`self.HighJumpActive` true)
  (`GameHud.HighJumpPowerupUpdates` (`GMRunner.GameHud` (`self.MainGameMode`)) 0.0 (`self.HighJump`)))

(event `/Game/Main/BP/interface/BPI_Player.DeactiveHighJump`
  (`self.HighJumpActive` false))

(event `/Game/Main/BP/interface/BPI_Player.ShieldPowerup`
  (`self.As BP Shield`
    (:`then`
      _)
    (:`else`
      (bind _asbp_shield (cast `/Game/Main/BP/Powerup/BP_Shield` (`ChildActorComponent.ChildActor` (`self.BP_Shield`))))
      (set `self.As BP Shield` _asbp_shield)))
  (`/Game/Main/BP/Powerup/BP_Shield.ShieldActive` (`self.As BP Shield`) true)
  (`SceneComponent.SetHiddenInGame` (`self.BP_Shield`) false false)
  (`GameHud.ShieldPowerupUpdates` (`GMRunner.GameHud` (`self.MainGameMode`)) 0.0 (`self.ShieldDuration`)))

(event `/Game/Main/BP/interface/BPI_Player.DeactiveShield`
  (`SceneComponent.SetHiddenInGame` (`self.BP_Shield`) true false)
  (`/Game/Main/BP/Powerup/BP_Shield.ShieldActive` (`self.As BP Shield`) false))

(fn `Character`
  (bind _returnvalue (`GameplayStatics.DoesSaveGameExist` "Menu"))
  (if _returnvalue
    (bind _returnvalue_2 (`GameplayStatics.LoadGameFromSlot` "Menu"))
    (bind _assv_game (cast `/Game/Main/BP/GameMode/SaveGame/SV_Game` _returnvalue_2))
    (`SkeletalMeshComponent.SetSkeletalMeshAsset` (`self.Mesh`) (`|GetArrayItem` (`self.CharacterMesh`) (`/Game/Main/BP/GameMode/SaveGame/SV_Game.SaveCharacterIndex` _assv_game)))
    (else
      (`SkeletalMeshComponent.SetSkeletalMeshAsset` (`self.Mesh`) (`|GetArrayItem` (`self.CharacterMesh`))))))

(fn `mesh&CapulseHeight`
  (params (Alpha :type "Float (double-precision)") (Alpha2 :type "Float (double-precision)"))
  (`CapsuleComponent.SetCapsuleHalfHeight` (`self.CapsuleComponent`) (`KismetMathLibrary.Lerp` 88.0 44.0 Alpha2) true)
  (`SceneComponent.K2_SetRelativeLocation` (`self.Mesh`) (`KismetMathLibrary.MakeVector` 0.0 0.0 (`KismetMathLibrary.Lerp` -90.0 -30.0 Alpha)) false false))

(fn `UserConstructionScript`)