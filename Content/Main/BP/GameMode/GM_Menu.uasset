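; GM_Menu is the main menu game mode that sets up the menu screen and shows saved currency.
; On BeginPlay it plays background music, adds the WI_Menu widget and shows the mouse cursor.
; It then loads the GameSlot save as SV_Game and sends saved coins and gems to every BP_CoinsMenu actor through the BPI_Communication interface, printing a failure message if no save exists.
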(event `self.ReceiveBeginPlay`
  (bind _gameslot (`self.GameSlot`))
  (`GameplayStatics.PlaySound2D` "/Game/Main/BP/HitSound/BackgroundMuisc.BackgroundMuisc" 1.0 1.0 0.0 null null)
  (bind _returnvalue (`|CreateWidget` "/Game/Main/BP/Widget/Menu/WI_Menu.WI_Menu_C"))
  (`UserWidget.AddToViewport` _returnvalue 0)
  (set `PlayerController.bShowMouseCursor` true (`GameplayStatics.GetPlayerController` 0))
  (bind _returnvalue_2 (`GameplayStatics.DoesSaveGameExist` _gameslot))
  (if _returnvalue_2
    (bind _returnvalue_3 (`GameplayStatics.LoadGameFromSlot` _gameslot))
    (bind _assv_game (cast `/Game/Main/BP/GameMode/SaveGame/SV_Game` _returnvalue_3))
    (bind _output_get (set `self.SaveMenuCoin` (`/Game/Main/BP/GameMode/SaveGame/SV_Game.SaveCoin` _assv_game)))
    (bind _output_get_2 (set `self.SaveMenuGems` (`/Game/Main/BP/GameMode/SaveGame/SV_Game.SaveGems` _assv_game)))
    (bind _outactors (`GameplayStatics.GetAllActorsOfClass` "/Game/Main/BP/Coins/BP_CoinsMenu.BP_CoinsMenu_C"))
    (for _array_element _outactors
      (if (`KismetSystemLibrary.DoesImplementInterface` _array_element "/Game/Main/BP/interface/BPI_Communication.BPI_Communication_C")
        (message `/Game/Main/BP/interface/BPI_Communication.CoinUpdate` _array_element _output_get _output_get_2)))
    (else
      (`KismetSystemLibrary.PrintString` "Fail"))))

(fn `UserConstructionScript`)