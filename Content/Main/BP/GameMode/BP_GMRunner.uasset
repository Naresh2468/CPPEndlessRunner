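; BP_GMRunner is the runner game mode Blueprint that persists coins, gems and high score.
; Saving loads or creates an SV_Game object in GameSlot, adding run totals to stored coins and gems and keeping the higher score.
; Small helper functions compute the merged values for existing saves.
; High score loading caches the stored value and passes it to GameHud, printing a failure message when no save exists.
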(event `self.SaveGameCall`
  (`self.SaveGameBP`))

(event `SaveGameBP`
  (bind _gameslot (`self.GameSlot`))
  (bind _totalcurrentscore (`self.TotalCurrentScore`))
  (bind _returnvalue (`GameplayStatics.DoesSaveGameExist` _gameslot))
  (if _returnvalue
    (bind _returnvalue_2 (`GameplayStatics.LoadGameFromSlot` _gameslot))
    (bind _assv_game (cast `/Game/Main/BP/GameMode/SaveGame/SV_Game` _returnvalue_2))
    (set `/Game/Main/BP/GameMode/SaveGame/SV_Game.SaveCoin` (`self.SaveCoin` _assv_game) _assv_game)
    (set `/Game/Main/BP/GameMode/SaveGame/SV_Game.SaveGems` (`self.SaveGems` _assv_game) _assv_game)
    (set `/Game/Main/BP/GameMode/SaveGame/SV_Game.SaveHighScore` (`self.CheckigScore` _assv_game) _assv_game)
    (`GameplayStatics.SaveGameToSlot` _assv_game (`self.GameSlot`))
    (else
      (bind _returnvalue_3 (`GameplayStatics.CreateSaveGameObject` "/Game/Main/BP/GameMode/SaveGame/SV_Game.SV_Game_C"))
      (set `/Game/Main/BP/GameMode/SaveGame/SV_Game.SaveCoin` (`self.TotalCoins`) _returnvalue_3)
      (set `/Game/Main/BP/GameMode/SaveGame/SV_Game.SaveGems` (`self.TotalGems`) _returnvalue_3)
      (bind _savehighscore (`/Game/Main/BP/GameMode/SaveGame/SV_Game.SaveHighScore` _returnvalue_3))
      (set `/Game/Main/BP/GameMode/SaveGame/SV_Game.SaveHighScore` (select `bool` (> _totalcurrentscore _savehighscore) :`false` _savehighscore :`true` _totalcurrentscore) _returnvalue_3)
      (`GameplayStatics.SaveGameToSlot` _returnvalue_3 (`self.GameSlot`)))))

(event `self.LoadHighscoreCall`
  (bind _gameslot (`self.GameSlot`))
  (bind _returnvalue (`GameplayStatics.DoesSaveGameExist` _gameslot))
  (if _returnvalue
    (bind _returnvalue_2 (`GameplayStatics.LoadGameFromSlot` _gameslot))
    (bind _assv_game (cast `/Game/Main/BP/GameMode/SaveGame/SV_Game` _returnvalue_2))
    (bind _savehighscore (`/Game/Main/BP/GameMode/SaveGame/SV_Game.SaveHighScore` _assv_game))
    (set `self.TotalHighScore` _savehighscore)
    (`GameHud.LoadHighScore` (`self.GameHud`) _savehighscore)
    (else
      (`KismetSystemLibrary.PrintString` "Fail"))))

(fn `UserConstructionScript`)