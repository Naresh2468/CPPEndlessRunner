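; A coin pickup actor (dark gold variant, by its name) that the player collects on touch and that supports magnet attraction.
; Overlapping its Box sends CoinCollectionsMessage to the player and game mode, plays the coin sound and destroys the coin.
; Overlapping CoinMagnetAttractionC while BP_Player's magnet is active starts a timeline that moves the coin toward the player using VInterpTo plus an animated vector offset.
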(event `self.Box.OnComponentBeginOverlap`
  (params (OverlappedComponent :type "PrimitiveComponent Object Reference") (OtherActor :type "Actor Object Reference") (OtherComp :type "PrimitiveComponent Object Reference") (OtherBodyIndex :type Integer) (bFromSweep :type Boolean) (SweepResult :type "HitResult Structure (by ref)"))
  (if (== OtherActor (`GameplayStatics.GetPlayerCharacter` 0))
    (message `/Game/GameEndless/Blueprint/Interface/I_MainGame.CoinCollections` OtherActor 0.0)
    (message `/Game/GameEndless/Blueprint/Interface/I_MainGame.CoinCollections` (`GameplayStatics.GetGameMode`) 0.0)
    (`GameplayStatics.PlaySoundAtLocation` "/Game/GameEndless/Audio/coin.coin" (`self.K2_GetActorLocation`) (struct) 1.0 1.0 0.0 null null null null)
    (`self.K2_DestroyActor`)))

(event `self.CoinMagnetAttractionC.OnComponentBeginOverlap`
  (params (OverlappedComponent :type "PrimitiveComponent Object Reference") (OtherActor :type "Actor Object Reference") (OtherComp :type "PrimitiveComponent Object Reference") (OtherBodyIndex :type Integer) (bFromSweep :type Boolean) (SweepResult :type "HitResult Structure (by ref)"))
  (if (== OtherActor (`GameplayStatics.GetPlayerCharacter` 0))
    (bind _asbp_player (cast `/Game/GameEndless/Blueprint/Players/BP_Player` OtherActor))
    (if (`/Game/GameEndless/Blueprint/Players/BP_Player.IsMagnetActive?` _asbp_player)
      (bind (_direction _magentvector) (`Timeline|MagneticAttractionTime` :!via `PlayFromStart`)
        (:`Update`
          (`self.K2_SetActorLocation` (+ _magentvector (`KismetMathLibrary.VInterpTo` (.location (`self.GetTransform`)) (`self.K2_GetActorLocation` (`GameplayStatics.GetPlayerCharacter` 0)) (`GameplayStatics.GetWorldDeltaSeconds`) 10.0))))))))

(fn `UserConstructionScript`)