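; Gold coin pickup that the player collects on overlap, with optional magnet attraction.
; The box overlap sends coin-collection messages to the player and the game mode, passing the coin's value to the latter, then plays a sound and destroys the coin.
; A second magnet overlap checks the player's IsMagnetActive flag and starts a timeline that pulls the coin toward the player with VInterpTo plus a vector-track offset.
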(event `self.Box.OnComponentBeginOverlap`
  (params (OverlappedComponent :type "PrimitiveComponent Object Reference") (OtherActor :type "Actor Object Reference") (OtherComp :type "PrimitiveComponent Object Reference") (OtherBodyIndex :type Integer) (bFromSweep :type Boolean) (SweepResult :type "HitResult Structure (by ref)"))
  (if (== OtherActor (`GameplayStatics.GetPlayerCharacter` 0))
    (message `/Game/Main/Ref/Coins/Bp_CoinsGold.CoinCollections` OtherActor 0.0)
    (message `/Game/Main/Ref/Coins/Bp_CoinsGold.CoinCollections` (`GameplayStatics.GetGameMode`) 10.0)
    (`GameplayStatics.PlaySoundAtLocation` null (`self.K2_GetActorLocation`) (struct) 1.0 1.0 0.0 null null null null)
    (`self.K2_DestroyActor`)))

(event `self.CoinMagnetAttractionC.OnComponentBeginOverlap`
  (params (OverlappedComponent :type "PrimitiveComponent Object Reference") (OtherActor :type "Actor Object Reference") (OtherComp :type "PrimitiveComponent Object Reference") (OtherBodyIndex :type Integer) (bFromSweep :type Boolean) (SweepResult :type "HitResult Structure (by ref)"))
  (if (== OtherActor (`GameplayStatics.GetPlayerCharacter` 0))
    (bind _asbp_player (cast `` OtherActor))
    (if (`/Game/Main/Ref/Coins/Bp_CoinsGold.IsMagnetActive?` _asbp_player)
      (bind (_direction _magentvector) (`Timeline|MagneticAttractionTime` :!via `PlayFromStart`)
        (:`Update`
          (`self.K2_SetActorLocation` (+ _magentvector (`KismetMathLibrary.VInterpTo` (.location (`self.GetTransform`)) (`self.K2_GetActorLocation` (`GameplayStatics.GetPlayerCharacter` 0)) (`GameplayStatics.GetWorldDeltaSeconds`) (`self.Interp Speed`)))))))))

(fn `UserConstructionScript`)