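; Brass coin pickup that the player collects by touching its box trigger.
; On overlap it sends CoinCollectionsMessage to both the player and the game mode with different values, plays a coin sound and destroys itself.
; A timeline-driven magnet pull toward the player exists but is disconnected, so the magnet overlap and BeginPlay events do nothing.
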(event `self.ReceiveBeginPlay`)

(event `self.Box.OnComponentBeginOverlap`
  (params (OverlappedComponent :type "PrimitiveComponent Object Reference") (OtherActor :type "Actor Object Reference") (OtherComp :type "PrimitiveComponent Object Reference") (OtherBodyIndex :type Integer) (bFromSweep :type Boolean) (SweepResult :type "HitResult Structure (by ref)"))
  (if (== OtherActor (`GameplayStatics.GetPlayerCharacter` 0))
    (message `/Game/GameEndless/Blueprint/Interface/I_MainGame.CoinCollections` OtherActor 0.0)
    (message `/Game/GameEndless/Blueprint/Interface/I_MainGame.CoinCollections` (`GameplayStatics.GetGameMode`) 10.0)
    (`GameplayStatics.PlaySoundAtLocation` "/Game/GameEndless/Audio/coin.coin" (`self.K2_GetActorLocation`) (struct) 1.0 1.0 0.0 null null null null)
    (`self.K2_DestroyActor`)))

(event `self.CoinMagnetAttractionC.OnComponentBeginOverlap`
  (params (OverlappedComponent :type "PrimitiveComponent Object Reference") (OtherActor :type "Actor Object Reference") (OtherComp :type "PrimitiveComponent Object Reference") (OtherBodyIndex :type Integer) (bFromSweep :type Boolean) (SweepResult :type "HitResult Structure (by ref)")))

(fn `UserConstructionScript`)