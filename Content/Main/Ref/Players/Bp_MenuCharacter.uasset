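; Menu-scene character that creates the I_Menu widget on BeginPlay and lets the player look around the menu.
; Horizontal and vertical look axes rotate the controller only while the menu's IsCamera and CameraHeadMove flags are on, tracked in IsCameraMENU.
; Custom events add a background audio component and stop it once the menu's PlayGame flag is set.
; Swipe look, spring-arm zoom and camera reset logic remain in the graph but are disconnected.
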(event `PlayBackgroundSound`
  (bind _returnvalue (`AddComponent|NODE_AddAudioComponent-0`))
  (set `self.Auido` _returnvalue))

(event `self.ReceiveBeginPlay`
  (bind _ref_menumanager (`self.Ref_MenuManager`))
  (bind _returnvalue (`|CreateWidget` "/Game/GameEndless/Blueprint/UI/I_Menu.I_Menu_C"))
  (bind _output_get (set `self.Ref_MenuManager` _returnvalue))
  (`UserWidget.AddToViewport` _output_get 0)
  (set `/Game/GameEndless/Blueprint/UI/I_Menu.IsCamera?` false _ref_menumanager)
  (set `/Game/GameEndless/Blueprint/UI/I_Menu.CameraHeadMove` false _ref_menumanager))

(event `StopAudio`
  (if (`/Game/GameEndless/Blueprint/UI/I_Menu.PlayGame?` (`self.Ref_MenuManager`))
    (`AudioComponent.Stop` (`self.Auido`))))

(event `InputTouch`
  (params (Location :type "Vector Structure") (FingerIndex :type "ETouchIndex Enum")))

(event `InputAxis|LookHorizontal`
  (params (AxisValue :type "Float (single-precision)"))
  (bind _ref_menumanager (`self.Ref_MenuManager`))
  (if (and (`/Game/GameEndless/Blueprint/UI/I_Menu.IsCamera?` _ref_menumanager) (`/Game/GameEndless/Blueprint/UI/I_Menu.CameraHeadMove` _ref_menumanager))
    (set `self.IsCameraMENU?` true)
    (`self.AddControllerYawInput` AxisValue)
    (else
      (set `self.IsCameraMENU?` false))))

(event `InputAxis|LookVertical`
  (params (AxisValue :type "Float (single-precision)"))
  (bind _ref_menumanager (`self.Ref_MenuManager`))
  (if (and (`/Game/GameEndless/Blueprint/UI/I_Menu.IsCamera?` _ref_menumanager) (`/Game/GameEndless/Blueprint/UI/I_Menu.CameraHeadMove` _ref_menumanager))
    (set `self.IsCameraMENU?` true)
    (`self.AddControllerPitchInput` AxisValue)
    (else
      (set `self.IsCameraMENU?` false))))

(event `InputAction|Zoom Mouse In`
  (params (Key :type "Key Structure")))

(event `InputAction|Zoom Mouse Out`
  (params (Key :type "Key Structure")))

(fn `UserConstructionScript`)