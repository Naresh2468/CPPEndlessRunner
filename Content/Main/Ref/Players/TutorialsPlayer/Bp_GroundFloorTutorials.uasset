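; Tutorial ground floor tile for a three-lane runner game.
; The construction script places the A6 and Dust components on one randomly chosen lane.
; When the player overlaps SpawnCollision, the tile calls GroundCallMessage on the game mode and destroys itself three seconds later.
; Helper functions for lane obstacle, coin and gem spawning remain, but nothing in this Blueprint calls them.
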(event `self.ReceiveBeginPlay`)

(event `self.SpawnCollision.OnComponentBeginOverlap`
  (params (OverlappedComponent :type "PrimitiveComponent Object Reference") (OtherActor :type "Actor Object Reference") (OtherComp :type "PrimitiveComponent Object Reference") (OtherBodyIndex :type Integer) (bFromSweep :type Boolean) (SweepResult :type "HitResult Structure (by ref)"))
  (if (== OtherActor (`GameplayStatics.GetPlayerCharacter` 0))
    (`|ExecutionSequence`
      (:`then_0`
        (message `/Game/GameEndless/Blueprint/Interface/I_MainGame.GroundCall` (`GameplayStatics.GetGameMode`)))
      (:`then_1`
        (`KismetSystemLibrary.Delay` 3.0)
        (`self.K2_DestroyActor`)))))

(event `self.SpawnCollision.OnComponentEndOverlap`
  (params (OverlappedComponent :type "PrimitiveComponent Object Reference") (OtherActor :type "Actor Object Reference") (OtherComp :type "PrimitiveComponent Object Reference") (OtherBodyIndex :type Integer)))

(fn `CoinSpawn`
  (bind _coinarea (`self.CoinArea`))
  (for _ (range 5)
    (`AddComponent|NODE_AddChildActorComponent-2` :`RelativeTransform` (`KismetMathLibrary.Conv_VectorToTransform` (+ (`KismetMathLibrary.RandomPointInBoundingBox` (`SceneComponent.RelativeLocation` _coinarea) (`BoxComponent.BoxExtent` _coinarea)) (0.0 0.0 30.0))))))

(fn `GemsSpawn`
  (bind _coinarea (`self.CoinArea`))
  (for _index (range 101)
    (if (< _index 1)
      (`AddComponent|NODE_AddChildActorComponent-3` :`RelativeTransform` (`KismetMathLibrary.Conv_VectorToTransform` (+ (`KismetMathLibrary.RandomPointInBoundingBox` (`SceneComponent.RelativeLocation` _coinarea) (`BoxComponent.BoxExtent` _coinarea)) (0.0 0.0 30.0)))))))

(fn `SpawnLocation`
  (set `self.SpawnPoint` (`|MakeArray` (`SceneComponent.GetRelativeTransform` (`self.LeftLane`)) (`SceneComponent.GetRelativeTransform` (`self.MiddleLane`)) (`SceneComponent.GetRelativeTransform` (`self.RightLane`)))))

(fn `SpawnObjects`
  (bind _spawnpoint (`self.SpawnPoint`))
  (`|ExecutionSequence`
    (:`then_0`
      (for _ (range 3)
        (`AddComponent|NODE_AddChildActorComponent-0` :`RelativeTransform` (`|GetArrayItem` _spawnpoint (`KismetMathLibrary.RandomIntegerInRange` 0 (`KismetArrayLibrary.Array_LastIndex` _spawnpoint))))))))

(fn `UserConstructionScript`
  (bind (_returnvalue_x _returnvalue_y) (`KismetMathLibrary.BreakVector` (`SceneComponent.K2_GetComponentLocation` (`self.LeftLane`))))
  (bind (_returnvalue_x_2 _returnvalue_y_2) (`KismetMathLibrary.BreakVector` (`SceneComponent.K2_GetComponentLocation` (`self.RightLane`))))
  (bind (_returnvalue_x_3 _returnvalue_y_3) (`KismetMathLibrary.BreakVector` (`SceneComponent.K2_GetComponentLocation` (`self.MiddleLane`))))
  (bind _output_get (set `self.NewVar` (`KismetArrayLibrary.Array_Random` (`|MakeArray` _returnvalue_y _returnvalue_y_2 _returnvalue_y_3))))
  (`SceneComponent.K2_SetRelativeLocation` (`self.a6`) (`KismetMathLibrary.MakeVector` 357.6 _output_get 59.8) false false)
  (`SceneComponent.K2_SetRelativeLocation` (`self.Dust`) (`KismetMathLibrary.MakeVector` 360.0 _output_get 50.0) false false))