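; Bp_Timers is a clock that counts elapsed seconds, minutes and hours during play.
; On BeginPlay it caches BP_Player and starts a looping one-second timer, whose event adds another one-second Delay before running the Timer function.
; Timer increments and rolls over the counters, though the hour rollover does not reset seconds.
; Each update also mirrors the player's SetTimerActive flag into SetTimerTextActive.
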(event `self.ReceiveBeginPlay`
  (bind _returnvalue (`GameplayStatics.GetActorOfClass` "/Game/GameEndless/Blueprint/Players/BP_Player.BP_Player_C"))
  (set `self.Bp_MAINPlayer` _returnvalue)
  (`KismetSystemLibrary.K2_SetTimerDelegate` (delegate `TimeStart`) 1.0 true))

(event `TimeStart`
  (`KismetSystemLibrary.Delay` 1.0)
  (`self.Timer`))

(fn `Timer`
  (bind _set_timer_active (`/Game/GameEndless/Blueprint/Players/BP_Player.Set Timer Active` (`self.Bp_MAINPlayer`)))
  (if (== (`self.SecT`) 59)
    (if (== (`self.MinsT`) 59)
      (set `self.MinsT` 0)
      (set `self.HRST` (+ (`self.HRST`) 1))
      (if _set_timer_active
        (set `self.SetTimerTextActive` true)
        (else
          (set `self.SetTimerTextActive` false)))
      (else
        (set `self.SecT` 0)
        (set `self.MinsT` (+ (`self.MinsT`) 1))
        (if _set_timer_active
          (set `self.SetTimerTextActive` true)
          (else
            (set `self.SetTimerTextActive` false)))))
    (else
      (set `self.SecT` (+ (`self.SecT`) 1))
      (if _set_timer_active
        (set `self.SetTimerTextActive` true)
        (else
          (set `self.SetTimerTextActive` false))))))

(fn `UserConstructionScript`)