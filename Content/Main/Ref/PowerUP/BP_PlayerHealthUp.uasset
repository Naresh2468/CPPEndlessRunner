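; BP_PlayerHealthUp is a health pickup that restores a random amount of health to the player on overlap.
; On BeginPlay it caches the BP_Player character and GM_Runner game mode.
; When the player overlaps HealthUpC, it adds a random value within its min/max range, clamped between zero and a hundred.
; It then updates the health bar and power-effect message through the game mode, prints a debug string and destroys itself.
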(event `self.ReceiveBeginPlay`
  (bind _asbp_player (cast `/Game/GameEndless/Blueprint/Players/BP_Player` (`GameplayStatics.GetPlayerCharacter` 0)))
  (set `self.As BP Player` _asbp_player)
  (bind _asgm_runner (cast `/Game/GameEndless/Blueprint/GameMode/GM_Runner` (`GameplayStatics.GetGameMode`)))
  (set `self.As GM Runner` _asgm_runner))

(event `self.HealthUpC.OnComponentBeginOverlap`
  (params (OverlappedComponent :type "PrimitiveComponent Object Reference") (OtherActor :type "Actor Object Reference") (OtherComp :type "PrimitiveComponent Object Reference") (OtherBodyIndex :type Integer) (bFromSweep :type Boolean) (SweepResult :type "HitResult Structure (by ref)"))
  (bind _as_bp_player (`self.As BP Player`))
  (bind _as_gm_runner (`self.As GM Runner`))
  (if (== OtherActor (`GameplayStatics.GetPlayerCharacter` 0))
    (bind _output_get (set `/Game/GameEndless/Blueprint/Players/BP_Player.PlayerHealth` (`KismetMathLibrary.FClamp` (+ (`/Game/GameEndless/Blueprint/Players/BP_Player.PlayerHealth` _as_bp_player) (`KismetMathLibrary.RandomFloatInRange` (`self.HealthUpMin`) (`self.HealthUpMax`))) 0.0 100.0) _as_bp_player))
    (`/Game/GameEndless/Blueprint/GameMode/GM_Runner.HealthBarI` _as_gm_runner _output_get)
    (message `/Game/GameEndless/Blueprint/Interface/I_MainGame.PowerActiveEffect` _as_gm_runner 0)
    (`KismetSystemLibrary.PrintString` (`self.Get Message` (`KismetStringLibrary.Conv_DoubleToString` _output_get)))
    (`self.K2_DestroyActor`)))

(fn `UserConstructionScript`)