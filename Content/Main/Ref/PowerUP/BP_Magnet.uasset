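; BP_Magnet is a magnet power-up pickup that the player collects by overlapping it.
; On MagnetCollision overlap with player character 0, it casts the actor, sets its IsMagnetActive flag and calls PlayerMagnet on it.
; It then prints a debug message citing an 8-second magnet duration and destroys itself, leaving the effect's behavior to the player character.
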(event `self.MagnetCollision.OnComponentBeginOverlap`
  (params (OverlappedComponent :type "PrimitiveComponent Object Reference") (OtherActor :type "Actor Object Reference") (OtherComp :type "PrimitiveComponent Object Reference") (OtherBodyIndex :type Integer) (bFromSweep :type Boolean) (SweepResult :type "HitResult Structure (by ref)"))
  (if (== OtherActor (`GameplayStatics.GetPlayerCharacter` 0))
    (bind _asbp_player (cast `` OtherActor))
    (set `/Game/Main/Ref/PowerUP/BP_Magnet.IsMagnetActive?` true _asbp_player)
    (`self.PlayerMagnet` _asbp_player)
    (`KismetSystemLibrary.PrintString` (`KismetStringLibrary.Concat_StrStr` (`KismetSystemLibrary.GetDisplayName` self) "Magnet active  for 8 sec") true true (struct :`R` 1.0 :`G` 0.166704 :`A` 1.0))
    (`self.K2_DestroyActor`)))

(fn `UserConstructionScript`)