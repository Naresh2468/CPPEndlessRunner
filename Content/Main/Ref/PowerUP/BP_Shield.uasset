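; BP_Shield is a shield power-up pickup that the player collects by touching it.
; When the player character overlaps its PowerupCollide component, it sets the shield-active flag on BP_Player and calls the player's shield power message.
; It then prints a debug string and destroys itself.
; The pickup has no timer of its own; the 8-second duration appears only in the printed text.
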(event `self.PowerupCollide.OnComponentBeginOverlap`
  (params (OverlappedComponent :type "PrimitiveComponent Object Reference") (OtherActor :type "Actor Object Reference") (OtherComp :type "PrimitiveComponent Object Reference") (OtherBodyIndex :type Integer) (bFromSweep :type Boolean) (SweepResult :type "HitResult Structure (by ref)"))
  (if (== OtherActor (`GameplayStatics.GetPlayerCharacter` 0))
    (bind _asbp_player (cast `/Game/GameEndless/Blueprint/Players/BP_Player` OtherActor))
    (set `/Game/GameEndless/Blueprint/Players/BP_Player.IsSheildActive` true _asbp_player)
    (message `/Game/GameEndless/Blueprint/Interface/I_MainGame.PlayerShieldPower` _asbp_player)
    (`KismetSystemLibrary.PrintString` (`self.SelfObjectName` "Shiedl_Up active  for 8 sec") true true (struct :`R` 0.215717 :`B` 1.0 :`A` 1.0))
    (`self.K2_DestroyActor`)))

(fn `UserConstructionScript`)