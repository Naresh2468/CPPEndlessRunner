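; BP_Hit_01 is a sphere effect actor whose material fade is toggled with the V key.
; A FlipFlop alternates between two timelines, each driving the "Fade" parameter on Sphere1's materials.
; The component hit event is empty; disconnected graphs hold an unused Niagara impact with an expanding material mask at the hit point, plus unused input enable/disable logic.
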(event `Key|V`
  (params (Key :type "Key Structure"))
  (bind _sphere1 (`self.Sphere1`))
  (:`Pressed`
    (`/Engine/EditorBlueprintResources/StandardMacros.FlipFlop`
      (:`A`
        (bind (_direction _posy) (`Timeline|Timeline_0` :!via `PlayFromStart`)
          (:`Update`
            (`MeshComponent.SetScalarParameterValueOnMaterials` _sphere1 "Fade" _posy))))
      (:`B`
        (bind (_direction_2 _posy_2) (`Timeline|Timeline_1` :!via `PlayFromStart`)
          (:`Update`
            (`MeshComponent.SetScalarParameterValueOnMaterials` _sphere1 "Fade" _posy_2)))))))

(event `self.Sphere1.OnComponentHit`
  (params (HitComponent :type "PrimitiveComponent Object Reference") (OtherActor :type "Actor Object Reference") (OtherComp :type "PrimitiveComponent Object Reference") (NormalImpulse :type "Vector Structure") (Hit :type "HitResult Structure (by ref)")))

(fn `UserConstructionScript`)